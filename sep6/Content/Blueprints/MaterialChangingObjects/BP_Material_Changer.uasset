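; BP_Material_Changer is an actor whose cube changes material while something overlaps its trigger box.
; Begin and end overlap on TriggerBox call events that set the cube's first material slot to NewMaterial or back to OriginalMaterial.
; It also caches its transform on BeginPlay and has events that teleport it to NewTransform or back to the original, though nothing in this graph calls them.
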(event OnComponentBeginOverlap(TriggerBox)
  (params (OverlappedComponent :type Primitive%20Component%20Object%20Reference) (OtherActor :type Actor%20Object%20Reference) (OtherComp :type Primitive%20Component%20Object%20Reference) (OtherBodyIndex :type Integer) (bFromSweep :type Boolean) (SweepResult :type Hit%20Result%20Structure%20%28by%20ref%29))
  (CallFunction|SwitchtoNewMaterial))

(event OnComponentEndOverlap(TriggerBox)
  (params (OverlappedComponent :type Primitive%20Component%20Object%20Reference) (OtherActor :type Actor%20Object%20Reference) (OtherComp :type Primitive%20Component%20Object%20Reference) (OtherBodyIndex :type Integer))
  (CallFunction|SwitchtoOriginalMaterial))

(event Custom|SwitchToNewMaterial
  (Rendering|Material|SetMaterial (Variables|Default|GetCube) 0 (Variables|Default|GetNewMaterial)))

(event Custom|Original%20Transform
  (Transformation|SetActorTransform (Variables|Default|GetOriginalTransform) false true))

(event Custom|SwitchToOriginalMaterial
  (Rendering|Material|SetMaterial (Variables|Default|GetCube) 0 (Variables|Default|GetOriginalMaterial)))

(event Custom|New%20Transform
  (Transformation|SetActorTransform (Variables|Default|GetNewTransform) false true))

(event Collision|EventActorBeginOverlap
  (params (OtherActor :type Actor%20Object%20Reference)))

(event EventTick
  (params (DeltaSeconds :type Float%20%28single-precision%29)))

(event EventBeginPlay
  (Variables|Default|SetOriginalTransform (Transformation|GetActorTransform)))

(fn ConstructionScript)