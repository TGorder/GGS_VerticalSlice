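; VisibilityEvent is a one-shot "back turned" actor that fires a surprise once the player has seen it and then looks away.
; For the desired character ID, Tick projects its location to screen and checks viewport bounds, with no occlusion test.
; Leaving view after being seen adds surprise text, then Fling sets the first "FlingMe"-tagged actor's location to its forward vector times 100, an absolute position.
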(event Custom|Fling
  (Transformation|SetActorLocation (Utilities|Array|Get(acopy) (stale EventTick _outactors)) (* (Transformation|GetActorForwardVector (Utilities|Array|Get(acopy) (stale EventTick _outactors))) 1e+02) false false)
  (Development|PrintString (Utilities|GetDisplayName (Utilities|Array|Get(acopy) (stale EventTick _outactors)))))

(event EventTick
  (params (DeltaSeconds :type Float%20%28single-precision%29))
  (bind _returnvalue (Transformation|GetActorLocation))
  (bind _returnvalue_2 (Game|GetPlayerController 0))
  (bind _screenlocation (Class|PlayerController|ProjectWorldLocationtoScreen _returnvalue_2 _returnvalue true))
  (bind (_sizex _sizey) (HUD|GetViewportSize _returnvalue_2))
  ;[1 1 1] Check If Actor is In Sight
  ;;[1 1 1] UPDATE
  ;;[1 1 1] Test if action has been performed
  (if (not (Variables|Default|GetactionPerformed))
    ;;[1 1 1] Test if player is desired character (default is investigator)
    (bind _asmy_game_instance (Utilities|Casting|CastToMyGameInstance (Game|GetGameInstance)))
    (if (== (Variables|/Game/GameModeStuff/MyGameInstance.MyGameInstance_C|GetCharacterID _asmy_game_instance) (Variables|Default|GetdesiredCharacterID))
      ;;[1 1 1] Test if actor is visible
      (if (Math|Boolean|ANDBoolean (> (.x _screenlocation) 0.0) (> (.y _screenlocation) 0.0) (< (.x _screenlocation) (Math|Conversions|ToFloat(Integer) _sizex)) (< (.y _screenlocation) (Math|Conversions|ToFloat(Integer) _sizey)))
        ;[1 1 1] If yes, test if the actor has already been seen
        (if (not (Variables|Default|GetwasSeen))
          ;[1 1 1] If not, set WasSeen to true
          (Variables|Default|SetwasSeen true)
          (Development|PrintString "Target seen" true true "(R=0.000000,G=0.660000,B=1.000000,A=1.000000)" 6e+01))
        (else
          ;[1 1 1] If no, test if the actor has already been seen
          (if (Variables|Default|GetwasSeen)
            ;[1 1 1] Test if the unique action has happened
            (if (not (Variables|Default|GetactionPerformed))
              ;[1 1 1] If not, perform the action
              (Variables|Default|SetactionPerformed true)
              (Development|PrintString "Action Performed" true true "(R=0.000000,G=0.660000,B=1.000000,A=1.000000)" 6e+01)
              ;[1 1 1] Add extra actions here
              (bind _returnvalue_3 (AddComponent|AddTextRenderComponent false (Math|Transform|MakeTransform "10.000000,50.000000,50.000000")))
              (Rendering|Components|TextRender|SetText _returnvalue_3 (Variables|Default|GetSurpriseText))
              (bind _outactors (Actor|GetAllActorswithTag "FlingMe"))
              (CallFunction|Fling))
            (else
              ;[1 1 1] Test if the first message has been shown
              (if (not (Variables|Default|GetfirstFailShown))
                ;[1 1 1] If not, show it
                (Variables|Default|SetfirstFailShown true)
                (Development|PrintString "Target has not yet been seen" true true "(R=0.000000,G=0.660000,B=1.000000,A=1.000000)" 6e+01)))))))))

(fn ConstructionScript)

(fn UniqueAction
  (params (NewParam1 :type Boolean))
  (return false))