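; Lever actor that the player flicks with F or a gamepad button to lock or unlock its assigned door.
; Overlapping InteractBox enables input and toggles an interaction widget, whose creation sits behind a DoOnce.
; The FlickSwitch timeline animates the roll forward or in reverse, then flips IsFlicked and calls LockDoor or UnlockDoor, only when DoorBP holds a single door.
; Flicking back to lock requires the door to be closed.
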(event OnComponentBeginOverlap(InteractBox)
  (params (OverlappedComponent :type Primitive%20Component%20Object%20Reference) (OtherActor :type Actor%20Object%20Reference) (OtherComp :type Primitive%20Component%20Object%20Reference) (OtherBodyIndex :type Integer) (bFromSweep :type Boolean) (SweepResult :type Hit%20Result%20Structure%20%28by%20ref%29))
  (Input|EnableInput (Game|GetPlayerController 0))
  ;[1 1 1] Create/Hide Interact Widget
  ;;[1 1 1] Test if widget is visible or not
  (if (Variables|Default|GetInteractionWidgetVisible)
    ;;[1 1 1] If it is, then remove it from the viewport and set bool to false
    (Widget|RemovefromParent (Variables|Default|GetInteractionWidget))
    (Variables|Default|SetInteractionWidgetVisible false)
    (else
      ;;[1 1 1] If not, show it
      (Utilities|FlowControl|DoOnce false
        (:Completed
          (bind _returnvalue (UserInterface|CreateWidget "/Game/Blueprints/ForReview/InteractionWidget.InteractionWidget_C" (Game|GetPlayerController 0)))
          (bind _output_get (Variables|Default|SetInteractionWidget _returnvalue))
          (UserInterface|Viewport|AddtoViewport _output_get 0)
          (Variables|Default|SetInteractionWidgetVisible true))))))

(event OnComponentEndOverlap(InteractBox)
  (params (OverlappedComponent :type Primitive%20Component%20Object%20Reference) (OtherActor :type Actor%20Object%20Reference) (OtherComp :type Primitive%20Component%20Object%20Reference) (OtherBodyIndex :type Integer))
  (Input|DisableInput (Game|GetPlayerController 0))
  ;[1 1 1] Create/Hide Interact Widget
  ;;[1 1 1] Test if widget is visible or not
  (if (Variables|Default|GetInteractionWidgetVisible)
    ;;[1 1 1] If it is, then remove it from the viewport and set bool to false
    (Widget|RemovefromParent (Variables|Default|GetInteractionWidget))
    (Variables|Default|SetInteractionWidgetVisible false)
    (else
      ;;[1 1 1] If not, show it
      (Utilities|FlowControl|DoOnce false
        (:Completed
          (bind _returnvalue (UserInterface|CreateWidget "/Game/Blueprints/ForReview/InteractionWidget.InteractionWidget_C" (Game|GetPlayerController 0)))
          (bind _output_get (Variables|Default|SetInteractionWidget _returnvalue))
          (UserInterface|Viewport|AddtoViewport _output_get 0)
          (Variables|Default|SetInteractionWidgetVisible true))))))

(event EventBeginPlay
  (bind _returnvalue (Transformation|GetActorRotation))
  (bind (_roll _pitch _yaw) (Math|Rotator|BreakRotator _returnvalue))
  (bind (_roll_2 _pitch_2 _yaw_2) (Math|Rotator|BreakRotator _returnvalue))
  (if (Variables|Default|GetisFlicked)
    (Transformation|SetActorRotation (Math|Rotator|MakeRotator 45.0 _pitch _yaw))
    (else
      (Transformation|SetActorRotation (Math|Rotator|MakeRotator -45.0 _pitch_2 _yaw_2)))))

(event Input|KeyboardEvents|F
  (params (Key :type Key%20Structure :default "AnyKey"))
  (bind _returnvalue (Transformation|GetActorRotation))
  (bind _door_bp (Variables|Default|GetDoor_BP))
  (bind (_roll _pitch _yaw) (Math|Rotator|BreakRotator _returnvalue))
  (:Pressed
    ;[1 1 1] Check if lever is flicked down
    (if (Variables|Default|GetisFlicked)
      ;[1 1 1] Check if the Lever's Assigned door is closed
      (for _array_element (Variables|Default|GetDoor_BP)
        _)
      ;[1 1 1] If its closed, we allow the lever to lock again
      (if (Variables|/Game/Blueprints/Doors/Door_Blueprint.Door_Blueprint_C|GetisClosed _array_element)
        ;[1 1 1] If not, play it forward. If it is, play timeline back ward
        (bind _flick (Timeline|Flick%20Switch ReverseFromEnd)
          (:Update
            (Transformation|SetActorRelativeRotation (Math|Rotator|MakeRotator _flick _pitch _yaw)))
          (:Finished
            (for _array_element_2 _door_bp
              (if (< (Utilities|Array|LastIndex _door_bp) 1)
                ;[1 1 1] Check is the switch is already flicked
                (if (Variables|Default|GetisFlicked)
                  (Variables|Default|SetisFlicked false)
                  ;[1 1 1] If it is, lock the door again
                  (Default|LockDoor _array_element_2)
                  (Development|PrintString "Locking door" true true "(R=0.965000,G=0.047613,B=0.009206,A=1.000000)")
                  (else
                    (Variables|Default|SetisFlicked true)
                    ;[1 1 1] If not, unlock the target door (if any)
                    (Default|UnlockDoor _array_element_2)
                    (Development|PrintString "Unlocking door" true true "(R=0.032973,G=0.415000,B=0.000000,A=1.000000)")))))))
        (else
          (Development|PrintString "Door is open. Close it to lock." true true "(R=0.962442,G=1.000000,B=0.964752,A=1.000000)")))
      (else
        (Timeline|Flick%20Switch Play)))))

(event Input|GamepadEvents|GamepadFaceButtonLeft
  (params (Key :type Key%20Structure :default "AnyKey"))
  (bind _returnvalue (Transformation|GetActorRotation))
  (bind _door_bp (Variables|Default|GetDoor_BP))
  (bind (_roll _pitch _yaw) (Math|Rotator|BreakRotator _returnvalue))
  (:Pressed
    ;[1 1 1] Check if lever is flicked down
    (if (Variables|Default|GetisFlicked)
      ;[1 1 1] Check if the Lever's Assigned door is closed
      (for _array_element (Variables|Default|GetDoor_BP)
        _)
      ;[1 1 1] If its closed, we allow the lever to lock again
      (if (Variables|/Game/Blueprints/Doors/Door_Blueprint.Door_Blueprint_C|GetisClosed _array_element)
        ;[1 1 1] If not, play it forward. If it is, play timeline back ward
        (bind _flick (Timeline|Flick%20Switch ReverseFromEnd)
          (:Update
            (Transformation|SetActorRelativeRotation (Math|Rotator|MakeRotator _flick _pitch _yaw)))
          (:Finished
            (for _array_element_2 _door_bp
              (if (< (Utilities|Array|LastIndex _door_bp) 1)
                ;[1 1 1] Check is the switch is already flicked
                (if (Variables|Default|GetisFlicked)
                  (Variables|Default|SetisFlicked false)
                  ;[1 1 1] If it is, lock the door again
                  (Default|LockDoor _array_element_2)
                  (Development|PrintString "Locking door" true true "(R=0.965000,G=0.047613,B=0.009206,A=1.000000)")
                  (else
                    (Variables|Default|SetisFlicked true)
                    ;[1 1 1] If not, unlock the target door (if any)
                    (Default|UnlockDoor _array_element_2)
                    (Development|PrintString "Unlocking door" true true "(R=0.032973,G=0.415000,B=0.000000,A=1.000000)")))))))
        (else
          (Development|PrintString "Door is open. Close it to lock." true true "(R=0.962442,G=1.000000,B=0.964752,A=1.000000)")))
      (else
        (Timeline|Flick%20Switch Play)))))

(fn ConstructionScript)